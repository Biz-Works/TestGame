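; Survival stat component tracking its owner's health, stamina, food, water and temperature.
; Looping function-name timers drain food and water, regenerate stamina, and apply cross-effects: low food costs health, low water costs stamina, full levels grant regeneration.
; Weather events shift temperature, which drifts back to normal, while heat speeds water loss and cold speeds food loss.
; Damage reduces health, publishing death and delayed respawn through MyGameStateBase at zero.
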(event Custom|DamageEvent
  (params (DamagedActor :type Actor%20Object%20Reference) (Damage :type Float%20%28single-precision%29) (DamageType :type Damage%20Type%20Object%20Reference) (InstigatedBy :type Controller%20Object%20Reference) (DamageCauser :type Actor%20Object%20Reference))
  (bind _as_my_game_state_base (Variables|Default|GetAs%20My%20Game%20State%20Base))
  ;[1 1 1] Damage Event
  (Variables|Health|SetCurrent%20Health (Math|Float|Clamp(Float) (- (Variables|Health|GetCurrent%20Health) Damage) 0.0 (Variables|Health|GetMaxHealth)))
  (if (<= (Variables|Health|GetCurrent%20Health) 0.0)
    (Variables|Health|SetDead? true)
    (Default|PublishonDeath _as_my_game_state_base)
    (Utilities|FlowControl|Delay 2.0)
    (Default|PublishonRespawn _as_my_game_state_base)))

(event Custom|Event%20Stamina%20Used
  ;[1 1 1] Event Use Stamina
  (if (> (Variables|Stamina|GetCurrentStamina) 0.0)
    (Variables|Stamina|SetOutofStamina? false)
    (else
      (Variables|Stamina|SetOutofStamina? true)))
  (if (Variables|Stamina|GetOutofStamina?)
    (if (>= (Variables|Stamina|GetCurrentStamina) 25.0)
      (Variables|Stamina|SetOutofStamina? false))
    (else
      (Utilities|FlowControl|DoOnce false :!label _label
        (:Completed
          (Variables|Stamina|SetCurrentStamina (Math|Float|Clamp(Float) (- (Variables|Stamina|GetCurrentStamina) 0.5) 0.0 1e+02))
          (if (<= (Variables|Stamina|GetCurrentStamina) 0.0)
            (Variables|Stamina|SetOutofStamina? true)
            (goto _label Reset)
            (else
              (Utilities|FlowControl|Delay 0.1)
              (goto _label Reset))))))))

(event Custom|Reset%20Timers
  ;[1 1 1] Restart Food Water Drain
  (Utilities|Time|SetTimerbyFunctionName 0 "FoodWaterDrain" 1e+01 true))

(event Custom|WarmWeather
  ;[1 1 1] TempChange
  (Utilities|Time|SetTimerbyFunctionName 0 "TempRaise" 1.0 true))

(event Custom|ColdWeather
  ;[1 1 1] TempChange
  (Utilities|Time|SetTimerbyFunctionName 0 "TempDrain" 1.0 true))

(event Custom|StopTempRaise
  ;[1 1 1] TempChange
  (Utilities|Time|SetTimerbyFunctionName 0 "TempRaise" 0.0))

(event Custom|Stop%20Temp%20Drain
  ;[1 1 1] TempChange
  (Utilities|Time|SetTimerbyFunctionName 0 "TempDrain" 0.0))

(event EventBeginPlay
  (bind _asmy_game_state_base (Utilities|Casting|CastToMyGameStateBase (Game|GetGameState)))
  (Variables|Default|SetAs%20My%20Game%20State%20Base _asmy_game_state_base)
  ;[1 1 1] Set Init Stats
  (Variables|Stamina|SetCurrentStamina (Variables|Stamina|GetMaxStamina))
  (Variables|Health|SetCurrent%20Health (Variables|Health|GetMaxHealth))
  (Variables|Food|SetCurrentFood (Variables|Food|GetFull_Food))
  (Variables|Water|SetCurrentWater (Variables|Water|GetFullWater))
  ;[1 1 1] Damage Event
  (EventDispatchers|BindEventtoOnTakeAnyDamage (Components|GetOwner) (delegate Custom|DamageEvent))
  ;[1 1 1] Regen Stamina
  (Utilities|Time|SetTimerbyFunctionName 0 "RegenStamina" 1.0 true)
  ;[1 1 1] Food and Water Updates
  (Utilities|Time|SetTimerbyFunctionName 0 "FoodWaterDrain" 1e+01 true)
  (Utilities|Time|SetTimerbyFunctionName 0 "FoodWaterFUll_ThenRegen" 0.8 true)
  (Utilities|Time|SetTimerbyFunctionName 0 "FoodWaterLowCheck" 1.0 true)
  ;[1 1 1] Temp Updates
  (Utilities|Time|SetTimerbyFunctionName 0 "BringTempToNormal" 3.5 true)
  (Utilities|Time|SetTimerbyFunctionName 0 "CheckTemp_InRange" 1.0 true))

(fn RegenHealth
  (Variables|Health|SetCurrent%20Health (Math|Float|Clamp(Float) (+ (Variables|Health|GetCurrent%20Health) 5.0) 0.0 (Variables|Health|GetMaxHealth)))
  (return))

(fn RegenStamina
  (if (Variables|Stamina|GetStopStaminaRegen?)
    (return)
    (else
      (Variables|Stamina|SetCurrentStamina (Math|Float|Clamp(Float) (+ (Variables|Stamina|GetCurrentStamina) 1.0) 0.0 (Variables|Stamina|GetMaxStamina)))
      (if (>= (Variables|Stamina|GetCurrentStamina) 5.0)
        (Variables|Stamina|SetOutofStamina? false))
      (return))))

(fn FoodWaterDrain
  (Water|WaterDrain)
  (Food|FoodDrain)
  (return))

(fn FoodDrain
  (Variables|Food|SetCurrentFood (Math|Float|Clamp(Float) (- (Variables|Food|GetCurrentFood) (Variables|Food|GetFoodDrainAmount)) 0.0 (Variables|Food|GetFull_Food)))
  (return))

(fn WaterDrain
  (Variables|Water|SetCurrentWater (Math|Float|Clamp(Float) (- (Variables|Water|GetCurrentWater) (Variables|Water|GetWaterDrainAmount)) 0.0 (Variables|Water|GetFullWater)))
  (return))

(fn FoodLowCheck
  (if (<= (Variables|Food|GetCurrentFood) 25.0)
    (Health|HealthDrain))
  (return))

(fn HealthDrain
  (Variables|Health|SetCurrent%20Health (Math|Float|Clamp(Float) (- (Variables|Health|GetCurrent%20Health) (Variables|Health|GetHealthDrainAmount)) 0.0 (Variables|Health|GetMaxHealth)))
  (return))

(fn WaterLowCheck
  (if (<= (Variables|Water|GetCurrentWater) 25.0)
    (Variables|Stamina|SetStopStaminaRegen? true)
    (Stamina|StaminaDrain)
    (else
      (Variables|Stamina|SetStopStaminaRegen? false)))
  (return))

(fn StaminaDrain
  (Variables|Stamina|SetCurrentStamina (Math|Float|Clamp(Float) (- (Variables|Stamina|GetCurrentStamina) (Variables|Stamina|GetStaminaDrainAmount)) 0.0 (Variables|Stamina|GetMaxStamina)))
  (return))

(fn TempDrain
  (Development|PrintString "Temp Drain Active" true true "(R=1.000000,G=0.000000,B=0.000000,A=1.000000)")
  (bind _output_get (LocalVariables|SetTempNumber (* (- (Variables|Temp|GetCurrentTemp) 1.0) 10)))
  (bind _returnvalue (Temp|ClampTemp (Math|Conversions|ToFloat(Integer) (/ _output_get 10))))
  (Variables|Temp|SetCurrentTemp _returnvalue)
  (return))

(fn TempRaise
  (Development|PrintString "Temp Raise Active" true true "(R=1.000000,G=0.000000,B=0.000000,A=1.000000)")
  (bind _output_get (LocalVariables|SetTempNumber (* (+ (Variables|Temp|GetCurrentTemp) 1.0) 10)))
  (bind _returnvalue (Temp|ClampTemp (Math|Conversions|ToFloat(Integer) (/ _output_get 10))))
  (Variables|Temp|SetCurrentTemp _returnvalue)
  (return))

(fn BringTemptoNormal
  (bind _currenttemp (Variables|Temp|GetCurrentTemp))
  (bind _normaltemp (Variables|Temp|GetNormalTemp))
  (if (== (Variables|Temp|GetCurrentTemp) (Variables|Temp|GetNormalTemp))
    (return)
    (elif (< _currenttemp _normaltemp)
      (Temp|TempRaise)
      (return)
      (elif (> _currenttemp _normaltemp)
        (Temp|TempDrain)
        (return)
        (else
          (return))))))

(fn CheckTempinRange
  (if (not (== (Variables|Temp|GetCurrentTemp) (Variables|Temp|GetNormalTemp)))
    (if (> (Variables|Temp|GetCurrentTemp) (Variables|Temp|GetUpperTempRange))
      (Variables|Temp|SetHot? true)
      (Development|PrintString "You are Hot" true true "(R=1.000000,G=0.024906,B=0.000000,A=1.000000)")
      (Utilities|Time|SetTimerbyFunctionName 0 "WaterDrain" 1.0 true)
      (else
        (Variables|Temp|SetHot? false)
        (Utilities|Time|SetTimerbyFunctionName 0 "WaterDrain" 0.0)))
    (if (< (Variables|Temp|GetCurrentTemp) (Variables|Temp|GetLowerTempRange))
      (Variables|Temp|SetCold? true)
      (Development|PrintString "You are Cold" true true "(R=1.000000,G=0.000000,B=0.049349,A=1.000000)")
      (Utilities|Time|SetTimerbyFunctionName 0 "FoodDrain" 0.5 true)
      (return)
      (else
        (Variables|Temp|SetCold? false)
        (Utilities|Time|SetTimerbyFunctionName 0 "FoodDrain" 0.0)
        (return)))))

(fn ClampTemp
  (params (Value :type Float%20%28double-precision%29))
  (return (Math|Float|Clamp(Float) Value (Variables|Temp|GetTempBottom) (Variables|Temp|GetTempTop))))

(fn FullWaterRegenStamina
  (if (== (Variables|Water|GetCurrentWater) (Variables|Water|GetFullWater))
    (Stamina|RegenStamina)
    (return)
    (else
      (return))))

(fn FullFoodRegenHealth
  (if (== (Variables|Food|GetCurrentFood) (Variables|Food|GetFull_Food))
    (Health|RegenHealth)
    (return)
    (else
      (return))))

(fn FoodWaterFUllThenRegen
  (Water|FullWaterRegenStamina)
  (Food|FullFoodRegenHealth)
  (return))

(fn FoodWaterDrainTickCancel
  (if (and (== (Variables|Food|GetCurrentFood) (Variables|Food|GetFull_Food)) (== (Variables|Water|GetCurrentWater) (Variables|Water|GetFullWater)))
    (Utilities|Time|ClearTimerbyFunctionName 0 "FoodWaterDrain")
    (return)))

(fn FoodWaterLowCheck
  (Water|WaterLowCheck)
  (Food|FoodLowCheck)
  (return))