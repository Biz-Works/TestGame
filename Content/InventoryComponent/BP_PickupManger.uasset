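; BP_PickupManger is a pickup manager in the inventory component folder that relays item overlap and pickup events.
; OverlapItem and PickupItem pass item class and amount to PublishItemOverlap and PublishItemPickup.
; The FreeSlot and FreeStack checks are stubs that always return false.
; BeginPlay and construction are empty, and the GameState message calls, along with a next-tick delay, are unconnected.
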(event EventBeginPlay)

(event EventOverlapItem
  (params (ItemClass :type BP%20Master%20Item%20Class%20Reference) (Amount :type Integer))
  (CallFunction|PublishItemOverlap ItemClass Amount))

(event EventPickupItem
  (params (Item%20Class :type BP%20Master%20Item%20Class%20Reference) (Amount :type Integer))
  (CallFunction|PublishItemPickup Item%20Class Amount))

(fn ConstructionScript)

(fn FreeSlot?
  (return false))

(fn FreeStack?
  (params (ItemClass :type BP%20Master%20Item%20Class%20Reference))
  (return false))