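; BP_Master_Item is a base item Blueprint that handles being used from the inventory system.
; On BeginPlay it casts and caches the game state as MyGameStateBase.
; When used, it prints the item's name on screen and asks the game state to publish a remove-item message for its Index.
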(event Custom|EventOnUsed
  (Development|PrintString (Utilities|String|Append "You used " (Utilities|String|ToString(Text) (.name (Variables|Default|GetItemInfo)))) true false "(R=0.000000,G=0.000000,B=0.000000,A=1.000000)")
  (Class|BPIInventoryGamestate|PublishRemoveItem(Message) (Variables|Default|GetMy%20Game%20State%20Base) (Variables|Default|GetIndex)))

(event EventBeginPlay
  (bind _asmy_game_state_base (Utilities|Casting|CastToMyGameStateBase (Game|GetGameState)))
  (Variables|Default|SetMy%20Game%20State%20Base _asmy_game_state_base))

(fn ConstructionScript)