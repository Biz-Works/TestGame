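; Pickup actor for the inventory system that represents an item class and amount in the world, detected by a sphere.
; It publishes item overlap messages through the GameState on overlap begin, then publishes a pickup message and destroys itself on overlap end.
; A RestEvent handler updates the leftover amount or destroys the actor on negative values, but its GameState binding never runs.
; The FreeSlot and FreeStack checks are stubs returning false.
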(event OnComponentBeginOverlap(Sphere)
  (params (OverlappedComponent :type Primitive%20Component%20Object%20Reference) (OtherActor :type Actor%20Object%20Reference) (OtherComp :type Primitive%20Component%20Object%20Reference) (OtherBodyIndex :type Integer) (bFromSweep :type Boolean) (SweepResult :type Hit%20Result%20Structure%20%28by%20ref%29))
  ;[1 1 1] Overlap
  (Class|BPIInventoryGamestate|PublishItemOverlap(Message) (Game|GetGameState) (Variables|Default|GetItem%20Class) (Variables|Default|GetAmont)))

(event OnComponentEndOverlap(Sphere)
  (params (OverlappedComponent :type Primitive%20Component%20Object%20Reference) (OtherActor :type Actor%20Object%20Reference) (OtherComp :type Primitive%20Component%20Object%20Reference) (OtherBodyIndex :type Integer))
  ;[1 1 1] EndOverlap
  (Class|BPIInventoryGamestate|PublishItemPickup(Message) (Game|GetGameState) (Variables|Default|GetItem%20Class) (Variables|Default|GetAmont))
  (Actor|DestroyActor))

(event Custom|RestEvent
  (params (Rest :type Integer))
  ;[1 1 1] Bind on Rest Event
  (if (not (< Rest 0))
    (if (not (== Rest 0))
      (Variables|Default|SetAmont Rest))
    (else
      (Actor|DestroyActor))))

(event EventBeginPlay
  (Variables|Default|SetAmont (Variables|Default|GetAmont))
  ;[1 1 1] Cast to Gamestate
  (bind _asmy_game_state_base (Utilities|Casting|CastToMyGameStateBase (Game|GetGameState)))
  (Variables|Default|SetMy%20Game%20State%20Base _asmy_game_state_base)
  ;[1 1 1] Bind on Rest Event
  (Utilities|FlowControl|DelayUntilNextTick))

(fn ConstructionScript)

(fn FreeSlot?
  (return false))

(fn FreeStack?
  (params (ItemClass :type BP%20Master%20Item%20Class%20Reference))
  (return false))