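; Inventory component that stores items as class-and-amount slots, with stacking, splitting, swapping, using and dropping.
; MyGameStateBase serves as the event hub, delivering pickup and slot requests and receiving per-slot widget updates and pickup remainders.
; AddItem recursively fills free stacks, then empty slots; using an item briefly spawns its actor to fire EventOnUsed.
; Removal spawns a pickup at a random navigable point near the owner, retrying until one is found.
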(event Custom|EventOnItemPickup
  (params (ItemClass :type BP%20Master%20Item%20Class%20Reference) (Amount :type Integer))
  ;[1 1 1] Bind On Pickup Event
  (bind (_success_ _rest) (CallFunction|AddItem ItemClass Amount))
  (if _success_
    (Default|PublishRest (Variables|Default|GetMy%20Game%20State%20Base) _rest)))

(event Custom|EventOnItemOverlap
  (params (ItemClass :type BP%20Master%20Item%20Class%20Reference) (Amout :type Integer))
  ;[1 1 1] Bind On Overlap Event
  (Development|PrintString (Utilities|String|Append "You Overlaped     " (Utilities|String|ToString(Integer) Amout) (Utilities|String|Append "     " (Utilities|GetClassDisplayName ItemClass))) true true "(R=0.458333,G=0.162854,B=0.023478,A=1.000000)"))

(event Custom|Publish_Spawn_Inventory
  ;[1 1 1] Publish Spawn / Destroy Widget
  (Class|BPIWidgetGamestate|PublishWidgetSpawn(Message) (Variables|Default|GetMy%20Game%20State%20Base)))

(event Custom|Publish_DeSpawn_Inventory
  ;[1 1 1] Publish Spawn / Destroy Widget
  (Class|BPIWidgetGamestate|PublishWidgetDestroy(Message) (Variables|Default|GetMy%20Game%20State%20Base)))

(event Custom|Publish_Update_Slot_At_Index
  (params (Index :type Integer))
  ;[1 1 1] Publish Widget Update Event
  (Class|BPIWidgetGamestate|PublishWidgetUpdate(Message) (Variables|Default|GetMy%20Game%20State%20Base) Index))

(event Custom|UseItemAtIndex
  (params (Index :type Integer))
  (bind _slots (Variables|Default|GetSlots))
  (bind _output (Utilities|Array|Get(acopy) _slots Index))
  (bind _itemclass (Utilities|Struct|BreakS_Inv_Slot _output))
  ;[1 1 1] UseItemAtIndex
  (if (Utilities|IsValidClass _itemclass)
    (bind _returnvalue (Game|SpawnActorfromClass _itemclass (Math|Transform|MakeTransform "0, 0, 0" "0, 0, 0" "1.000000,1.000000,1.000000") "AlwaysSpawn" "MultiplyWithRoot" (Components|GetOwner) Index 0))
    (Default|EventonUsed _returnvalue)
    (Actor|DestroyActor _returnvalue)))

(event Custom|OnRemoveItem_Event
  (params (Index :type Integer))
  ;[1 1 1] Bind on Remove Item at Index
  (CallFunction|RemoveItematIndex Index 1))

(event Custom|OnUseItemAtIndex_Event
  (params (Index :type Integer))
  ;[1 1 1] Bind on Use Item at Index
  (CallFunction|UseItematIndex Index))

(event Custom|OnSplitStack_Event
  (params (Index :type Integer) (Amount :type Integer))
  ;[1 1 1] Bind on Split Stack
  (CallFunction|OnSplitStackEvent Index Amount))

(event Custom|OnSwapSlots_Event
  (params (Index%201 :type Integer) (Index%202 :type Integer))
  ;[1 1 1] Bind on Swap Stack
  (CallFunction|OnSwapSlotsEvent Index%201 Index%202))

(event EventBeginPlay
  (bind _asmy_game_state_base (Utilities|Casting|CastToMyGameStateBase (Game|GetGameState)))
  (Variables|Default|SetMy%20Game%20State%20Base _asmy_game_state_base)
  (Utilities|Array|Resize (Variables|Default|GetSlots) (Variables|Default|GetAmountofSlots))
  ;[1 1 1] Bind On Overlap Event
  (EventDispatchers|BindEventtoOnItemOverlap (Variables|Default|GetMy%20Game%20State%20Base) (delegate Custom|EventOnItemOverlap))
  ;[1 1 1] Bind On Pickup Event
  (EventDispatchers|BindEventtoOnItemPickup (Variables|Default|GetMy%20Game%20State%20Base) (delegate Custom|EventOnItemPickup))
  ;[1 1 1] Bind on Use Item at Index
  (EventDispatchers|AssignOnUseItematIndex (Variables|Default|GetMy%20Game%20State%20Base) (delegate Custom|OnUseItemAtIndex_Event))
  ;[1 1 1] Bind on Remove Item at Index
  (EventDispatchers|AssignOnRemoveItem (Variables|Default|GetMy%20Game%20State%20Base) (delegate Custom|OnRemoveItem_Event))
  ;[1 1 1] Bind on Split Stack
  (EventDispatchers|AssignOnSplitStack (Variables|Default|GetMy%20Game%20State%20Base) (delegate Custom|OnSplitStack_Event))
  ;[1 1 1] Bind on Swap Stack
  (EventDispatchers|AssignOnSwapSlots (Variables|Default|GetMy%20Game%20State%20Base) (delegate Custom|OnSwapSlots_Event)))

(fn IsSlotEmpty?
  (params (Index :type Integer))
  (return (not (Utilities|IsValidClass (.ItemClass (Utilities|Struct|BreakS_Inv_Slot (Utilities|Array|Get(acopy) (Variables|Default|GetSlots) Index)))))))

(fn GetAmountatIndex
  (params (Index :type Integer))
  (return (.Amount (Utilities|Struct|BreakS_Inv_Slot (Utilities|Array|Get(acopy) (Variables|Default|GetSlots) Index)))))

(fn GetItemInfoatIndex
  (params (Index :type Integer))
  (bind _slots (Variables|Default|GetSlots))
  (bind _output (Utilities|Array|Get(acopy) _slots Index))
  (bind (_itemclass _amount) (Utilities|Struct|BreakS_Inv_Slot _output))
  (if (Utilities|IsValidClass _itemclass)
    (return false (.ItemInfo (Utilities|GetClassDefaults _itemclass)) _amount)
    (else
      (return true "" 0))))

(fn RemoveItematIndex
  (params (Index :type Integer) (Amount :type Integer))
  (bind _slots (Variables|Default|GetSlots))
  (LocalVariables|SetLocal_Index Index)
  (LocalVariables|SetLocal_Amount Amount)
  (if (and (not (CallFunction|IsSlotEmpty? (LocalVariables|GetLocal_Index))) (> (LocalVariables|GetLocal_Amount) 0))
    (if (>= (LocalVariables|GetLocal_Amount) (CallFunction|GetAmountatIndex (LocalVariables|GetLocal_Index)))
      (CallFunction|SpawnDropedItem (LocalVariables|GetLocal_Index) (LocalVariables|GetLocal_Amount))
      (Utilities|Array|SetArrayElem (Variables|Default|GetSlots) (LocalVariables|GetLocal_Index) (Utilities|Struct|MakeS_Inv_Slot 0 0))
      (CallFunction|PublishUpdateSlotatIndex (LocalVariables|GetLocal_Index))
      (return true)
      (else
        (CallFunction|SpawnDropedItem (LocalVariables|GetLocal_Index) (- (.Amount (Utilities|Struct|BreakS_Inv_Slot (Utilities|Array|Get(acopy) (Variables|Default|GetSlots) (LocalVariables|GetLocal_Index)))) (LocalVariables|GetLocal_Amount)))
        (Utilities|Array|SetArrayElem _slots (LocalVariables|GetLocal_Index) (Utilities|Struct|MakeS_Inv_Slot (.ItemClass (Utilities|Struct|BreakS_Inv_Slot (Utilities|Array|Get(acopy) _slots (LocalVariables|GetLocal_Index)))) (- (.Amount (Utilities|Struct|BreakS_Inv_Slot (Utilities|Array|Get(acopy) _slots (LocalVariables|GetLocal_Index)))) (LocalVariables|GetLocal_Amount))))
        (CallFunction|PublishUpdateSlotatIndex (LocalVariables|GetLocal_Index))
        (return true)))
    (else
      (return false))))

(fn SearchEmptySlot
  (bind (_array_element _array_index) (Utilities|Array|ForEachLoopwithBreak (Variables|Default|GetSlots) :!label _label)
    (:LoopBody
      (if (not (Utilities|IsValidClass (.ItemClass (Utilities|Struct|BreakS_Inv_Slot _array_element))))
        (LocalVariables|SetLocalBool true)
        (LocalVariables|SetLocalIndex _array_index)
        (goto _label Break)))
    (:Completed
      (return (LocalVariables|GetLocalBool) (LocalVariables|GetLocalIndex)))))

(fn SearchFreeStack
  (params (ItemClass :type BP%20Master%20Item%20Class%20Reference))
  (bind (_array_element _array_index) (Utilities|Array|ForEachLoopwithBreak (Variables|Default|GetSlots) :!label _label)
    (:LoopBody
      (if (Utilities|IsValidClass (.ItemClass (Utilities|Struct|BreakS_Inv_Slot _array_element)))
        (if (and (== (.ItemClass (Utilities|Struct|BreakS_Inv_Slot _array_element)) ItemClass) (< (.Amount (Utilities|Struct|BreakS_Inv_Slot _array_element)) (Variables|Default|GetMaxStackSize)))
          (LocalVariables|SetLocalBool true)
          (LocalVariables|SetLocalIndex _array_index)
          (goto _label Break))))
    (:Completed
      (return (LocalVariables|GetLocalBool) (LocalVariables|GetLocalIndex)))))

(fn AddItem
  (params (Item%20Class :type BP%20Master%20Item%20Class%20Reference) (Amont :type Integer))
  (LocalVariables|SetLocalClass Item%20Class)
  (LocalVariables|SetLocalAmount Amont)
  (if (.CanBeStacked? (Utilities|Struct|BreakS_Item_info (.ItemInfo (Utilities|GetClassDefaults Item%20Class))))
    (bind (_success_ _index) (CallFunction|SearchFreeStack (LocalVariables|GetLocalClass)))
    (if _success_
      ;[1 1 1] Comment
      (LocalVariables|SetFoundIndex _index)
      (if (> (+ (.Amount (Utilities|Struct|BreakS_Inv_Slot (Utilities|Array|Get(acopy) (Variables|Default|GetSlots) (LocalVariables|GetFoundIndex)))) (LocalVariables|GetLocalAmount)) (Variables|Default|GetMaxStackSize))
        (LocalVariables|SetLocalAmount (- (+ (.Amount (Utilities|Struct|BreakS_Inv_Slot (Utilities|Array|Get(acopy) (Variables|Default|GetSlots) (LocalVariables|GetFoundIndex)))) (LocalVariables|GetLocalAmount)) (Variables|Default|GetMaxStackSize)))
        (Utilities|Array|SetArrayElem (Variables|Default|GetSlots) (LocalVariables|GetFoundIndex) (Utilities|Struct|MakeS_Inv_Slot (LocalVariables|GetLocalClass) (Variables|Default|GetMaxStackSize)))
        (CallFunction|PublishUpdateSlotatIndex (LocalVariables|GetFoundIndex))
        (bind _rest (CallFunction|AddItem (LocalVariables|GetLocalClass) (LocalVariables|GetLocalAmount)))
        (return true _rest)
        (else
          (Utilities|Array|SetArrayElem (Variables|Default|GetSlots) (LocalVariables|GetFoundIndex) (Utilities|Struct|MakeS_Inv_Slot (LocalVariables|GetLocalClass) (+ (.Amount (Utilities|Struct|BreakS_Inv_Slot (Utilities|Array|Get(acopy) (Variables|Default|GetSlots) (LocalVariables|GetFoundIndex)))) (LocalVariables|GetLocalAmount))))
          (CallFunction|PublishUpdateSlotatIndex (LocalVariables|GetFoundIndex))
          (return true 0)))
      (else
        ;[1 1 1] Comment
        (bind (_success__2 _index_2) (CallFunction|SearchEmptySlot))
        (if _success__2
          (LocalVariables|SetFoundIndex _index_2)
          (if (> (LocalVariables|GetLocalAmount) (Variables|Default|GetMaxStackSize))
            (Utilities|Array|SetArrayElem (Variables|Default|GetSlots) (LocalVariables|GetFoundIndex) (Utilities|Struct|MakeS_Inv_Slot (LocalVariables|GetLocalClass) (Variables|Default|GetMaxStackSize)))
            (CallFunction|PublishUpdateSlotatIndex (LocalVariables|GetFoundIndex))
            (bind _rest_2 (CallFunction|AddItem (LocalVariables|GetLocalClass) (- (LocalVariables|GetLocalAmount) (Variables|Default|GetMaxStackSize))))
            (return true _rest_2)
            (else
              (Utilities|Array|SetArrayElem (Variables|Default|GetSlots) (LocalVariables|GetFoundIndex) (Utilities|Struct|MakeS_Inv_Slot (LocalVariables|GetLocalClass) (LocalVariables|GetLocalAmount)))
              (CallFunction|PublishUpdateSlotatIndex (LocalVariables|GetFoundIndex))
              (return true 0)))
          (else
            (return false (LocalVariables|GetLocalAmount))))))
    (else
      ;[1 1 1] Comment
      (bind (_success__3 _index_3) (CallFunction|SearchEmptySlot))
      (if _success__3
        (LocalVariables|SetFoundIndex _index_3)
        (Utilities|Array|SetArrayElem (Variables|Default|GetSlots) (LocalVariables|GetFoundIndex) (Utilities|Struct|MakeS_Inv_Slot (LocalVariables|GetLocalClass) 1))
        (CallFunction|PublishUpdateSlotatIndex (LocalVariables|GetFoundIndex))
        (if (> (LocalVariables|GetLocalAmount) 1)
          (bind _rest_3 (CallFunction|AddItem (LocalVariables|GetLocalClass) (- (LocalVariables|GetLocalAmount) 1)))
          (return true _rest_3)
          (else
            (return true 0)))
        (else
          (return false (LocalVariables|GetLocalAmount)))))))

(fn SwapSlots
  (params (Index1 :type Integer) (Index2 :type Integer))
  (bind _slots (Variables|Default|GetSlots))
  (bind _returnvalue (Utilities|Array|LastIndex _slots))
  (LocalVariables|SetLocalIndex1 Index1)
  (LocalVariables|SetLocalIndex2 Index2)
  (if (or (> (LocalVariables|GetLocalIndex1) _returnvalue) (> (LocalVariables|GetLocalIndex2) _returnvalue))
    (return false)
    (else
      (LocalVariables|SetLocalSlot2 (Utilities|Array|Get(acopy) (Variables|Default|GetSlots) (LocalVariables|GetLocalIndex2)))
      (Utilities|Array|SetArrayElem (Variables|Default|GetSlots) (LocalVariables|GetLocalIndex2) (Utilities|Array|Get(acopy) (Variables|Default|GetSlots) (LocalVariables|GetLocalIndex1)))
      (Utilities|Array|SetArrayElem (Variables|Default|GetSlots) (LocalVariables|GetLocalIndex1) (LocalVariables|GetLocalSlot2))
      (CallFunction|PublishUpdateSlotatIndex (LocalVariables|GetLocalIndex1))
      (CallFunction|PublishUpdateSlotatIndex (LocalVariables|GetLocalIndex2))
      (return true))))

(fn SplitStack
  (params (StackIndex :type Integer) (Amount :type Integer))
  (bind _slots (Variables|Default|GetSlots))
  (LocalVariables|SetLocalStackIndex StackIndex)
  (LocalVariables|SetLocalAmount Amount)
  (if (CallFunction|IsSlotEmpty? (LocalVariables|GetLocalStackIndex))
    (return false)
    (elif (and (.CanBeStacked? (Utilities|Struct|BreakS_Item_info (.ItemInfo (CallFunction|GetItemInfoatIndex (LocalVariables|GetLocalStackIndex))))) (> (.Amount (CallFunction|GetItemInfoatIndex (LocalVariables|GetLocalStackIndex))) (LocalVariables|GetLocalAmount)))
      (bind (_success_ _index) (CallFunction|SearchEmptySlot))
      (if _success_
        (LocalVariables|SetLocalFoundIndex _index)
        (Utilities|Array|SetArrayElem _slots (LocalVariables|GetLocalStackIndex) (Utilities|Struct|MakeS_Inv_Slot (.ItemClass (Utilities|Struct|BreakS_Inv_Slot (Utilities|Array|Get(acopy) _slots (LocalVariables|GetLocalStackIndex)))) (- (.Amount (Utilities|Struct|BreakS_Inv_Slot (Utilities|Array|Get(acopy) _slots (LocalVariables|GetLocalStackIndex)))) (LocalVariables|GetLocalAmount))))
        (Utilities|Array|SetArrayElem (Variables|Default|GetSlots) (LocalVariables|GetLocalFoundIndex) (Utilities|Struct|MakeS_Inv_Slot (.ItemClass (Utilities|Struct|BreakS_Inv_Slot (Utilities|Array|Get(acopy) _slots (LocalVariables|GetLocalStackIndex)))) (LocalVariables|GetLocalAmount)))
        (CallFunction|PublishUpdateSlotatIndex (LocalVariables|GetLocalStackIndex))
        (CallFunction|PublishUpdateSlotatIndex (LocalVariables|GetLocalFoundIndex))
        (return true)
        (else
          (return false)))
      (else
        (return false)))))

(fn SpawnDropedItem
  (params (Index :type Integer) (Amount :type Integer))
  (bind (_randomlocation _returnvalue) (Class|NavigationSystemV1|GetRandomLocationinNavigableRadius (Transformation|GetActorLocation (Components|GetOwner)) 3.3e+02 0 0 :!label _label))
  (if _returnvalue
    (Game|SpawnActorfromClass "/Game/InventoryComponent/PickupActor/BP_Pickup_Actor.BP_Pickup_Actor_C" (Math|Transform|MakeTransform _randomlocation "0, 0, 0" "1.000000,1.000000,1.000000") "AlwaysSpawn" "MultiplyWithRoot" 0 (.ItemClass (Utilities|Struct|BreakS_Inv_Slot (Utilities|Array|Get(acopy) (Variables|Default|GetSlots) Index))) Amount 0)
    (return)
    (else
      (goto _label))))

(fn FreeSlot?
  (bind _freeslot_ (CallFunction|FreeSlot?))
  (return _freeslot_))

(fn FreeStack?
  (params (ItemClass :type BP%20Master%20Item%20Class%20Reference))
  (bind _success_ (CallFunction|SearchFreeStack ItemClass))
  (return _success_))