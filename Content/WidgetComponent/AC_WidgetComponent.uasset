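; AC_WidgetComponent is an actor component that creates the main HUD at BeginPlay and controls its inventory widget.
; It binds to widget spawned, destroyed and update events on MyGameStateBase, which acts as the dispatcher.
; Spawned and destroyed toggle the inventory's visibility and enabled state, mouse cursor and input mode, without creating or removing the widget.
; Update refreshes the inventory slot at the given index.
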(event Custom|OnWidgetSpawnedEvent
  (bind _returnvalue (Game|GetPlayerController 0))
  ;[1 1 1] Bind on Widget Spawned
  (Widget|SetVisibility (Variables|/Game/WidgetComponent/WBP_Main_Hud.WBP_Main_Hud_C|GetWBP_Inventory_Widget (Variables|Default|GetMainHud)) "Visible")
  (Input|SetInputModeGameandUI _returnvalue (Variables|Default|GetMainHud) "DoNotLock" true false)
  (Variables|/Script/Engine.PlayerController|SetbShowMouseCursor _returnvalue true)
  (Widget|SetIsEnabled (Variables|/Game/WidgetComponent/WBP_Main_Hud.WBP_Main_Hud_C|GetWBP_Inventory_Widget (Variables|Default|GetMainHud)) true))

(event Custom|OnWidgetDestroyed_Event
  (bind _returnvalue (Game|GetPlayerController 0))
  ;[1 1 1] Bind on widget Destroyed
  (Widget|SetVisibility (Variables|/Game/WidgetComponent/WBP_Main_Hud.WBP_Main_Hud_C|GetWBP_Inventory_Widget (Variables|Default|GetMainHud)) "Collapsed")
  (Input|SetInputModeGameOnly _returnvalue false)
  (Variables|/Script/Engine.PlayerController|SetbShowMouseCursor _returnvalue false)
  (Widget|SetIsEnabled (Variables|/Game/WidgetComponent/WBP_Main_Hud.WBP_Main_Hud_C|GetWBP_Inventory_Widget (Variables|Default|GetMainHud)) false))

(event Custom|OnWidgetUpdate_Event
  (params (Index :type Integer))
  ;[1 1 1] Bind On Update Widget
  (Default|UpdateSlot (Utilities|Array|Get(acopy) (Variables|/Game/InventoryComponent/Widgets/WBP_Inventory.WBP_Inventory_C|GetSlotsWidgets (Variables|/Game/WidgetComponent/WBP_Main_Hud.WBP_Main_Hud_C|GetWBP_Inventory_Widget (Variables|Default|GetMainHud))) Index)))

(event EventBeginPlay
  ;[1 1 1] Gamestate Cast
  (bind _asmy_game_state_base (Utilities|Casting|CastToMyGameStateBase (Game|GetGameState))
    (:then
      (Variables|Default|SetAs%20My%20Game%20State%20Base _asmy_game_state_base)
      ;[1 1 1] MainHudWidget
      (bind _returnvalue (UserInterface|CreateWidget "/Game/WidgetComponent/WBP_Main_Hud.WBP_Main_Hud_C" (Game|GetPlayerController 0)))
      (Variables|Default|SetMainHud _returnvalue)
      (UserInterface|Viewport|AddtoViewport (Variables|Default|GetMainHud) 0)
      ;[1 1 1] Bind on Widget Spawned
      (EventDispatchers|BindEventtoOnWidgetSpawned (Variables|Default|GetAs%20My%20Game%20State%20Base) (delegate Custom|OnWidgetSpawnedEvent))
      ;[1 1 1] Bind on widget Destroyed
      (EventDispatchers|AssignOnWidgetDestroyed (Variables|Default|GetAs%20My%20Game%20State%20Base) (delegate Custom|OnWidgetDestroyed_Event))
      ;[1 1 1] Bind On Update Widget
      (EventDispatchers|AssignOnWidgetUpdate (Variables|Default|GetAs%20My%20Game%20State%20Base) (delegate Custom|OnWidgetUpdate_Event)))
    (:CastFailed
      (Development|PrintString "Game state not valid in AC_WidgetComponent"))))